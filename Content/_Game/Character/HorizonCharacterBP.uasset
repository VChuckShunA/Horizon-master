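; HorizonCharacterBP is a character Blueprint that relays inventory, currency and vendor changes to the inventory UI.
; Its item event asks WInventory whether to add a new item, then either adds it or refreshes from the current inventory.
; Other events push coin totals and item lists to WInventory, or show and hide the VendorInventory panel in WInventoryUI.
; BeginPlay, Tick and the construction script are empty, and a controller cast is left unconnected.
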(event EventBeginPlay)

(event Collision|EventActorBeginOverlap
  (params (OtherActor :type Actor%20Object%20Reference)))

(event EventTick
  (params (DeltaSeconds :type Float%20%28single-precision%29)))

(event EventShowVendorInventory
  (params (Visible :type Boolean))
  (bind _w_inventory_ui (Variables|Default|GetW_Inventory_UI))
  (bind _vendorinventory (Variables|/Game/_Game/HUD/Inventory_UI.Inventory_UI_C|GetVendorInventory _w_inventory_ui))
  (Utilities|IsValid (Variables|Default|GetW_Inventory_UI)
    (:Is%20Valid
      (if Visible
        (Widget|SetVisibility _vendorinventory "Visible")
        (else
          (Widget|SetVisibility _vendorinventory "Hidden"))))))

(event EventUpdateCurrency
  (params (InventoryCoins :type Integer))
  (Default|UpdateCoins (Variables|Default|GetW_Inventory) InventoryCoins))

(event EventUpdateInventoryWidget
  (params (NewInventoryItems :type Array%20of%20Item%20Data%20Structures))
  (Default|Update (Variables|Default|GetW_Inventory) NewInventoryItems))

(event EventAddItemandUpdateInventoryWidget
  (params (ItemData :type Item%20Data%20Structure) (CurrentInventory :type Array%20of%20Item%20Data%20Structures))
  (bind _w_inventory (Variables|Default|GetW_Inventory))
  (bind _addnewitem (Default|ShouldAddNewItem _w_inventory CurrentInventory))
  (if _addnewitem
    (Default|AddItem (Variables|Default|GetW_Inventory) ItemData)
    (else
      (Default|Update _w_inventory CurrentInventory))))

(fn ConstructionScript)