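; BP_PickupTruck is a pickup truck Blueprint that manages the player's race HUD.
; On BeginPlay it creates Speedometer, Laps and WrongWay widgets and adds the speedometer, lap display and initially hidden warning to the viewport.
; Tick reads Backwards from the player's truck and, while it is 1, blinks the warning through a Delay and FlipFlop, otherwise hiding it.
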(event EventBeginPlay
  (bind _returnvalue (UserInterface|CreateWidget "/Game/_Game/VehicleSystem/Speedometer.Speedometer_C"))
  (UserInterface|Viewport|AddtoViewport _returnvalue 0)
  (bind _returnvalue_2 (UserInterface|CreateWidget "/Game/_Game/VehicleSystem/Laps.Laps_C"))
  (bind _returnvalue_3 (UserInterface|CreateWidget "/Game/_Game/VehicleSystem/WrongWay.WrongWay_C"))
  (Widget|SetVisibility _returnvalue_3 "Hidden")
  (UserInterface|Viewport|AddtoViewport _returnvalue_2 0))

(event Collision|EventActorBeginOverlap
  (params (OtherActor :type Actor%20Object%20Reference)))

(event EventTick
  (params (DeltaSeconds :type Float%20%28single-precision%29))
  (bind _asbp_pickup_truck (Utilities|Casting|CastToBP_PickupTruck (Game|Player|GetPlayerPawn 0)))
  (if (== (Variables|BP_PickupTruck_C|GetBackwards? _asbp_pickup_truck) 1)
    (Utilities|FlowControl|Delay 0.2)
    (Utilities|FlowControl|FlipFlop
      (:A
        (Widget|SetVisibility (stale EventBeginPlay _returnvalue_3) "Visible"))
      (:B
        (Widget|SetVisibility (stale EventBeginPlay _returnvalue_3) "Hidden")))
    (else
      (Widget|SetVisibility (stale EventBeginPlay _returnvalue_3) "Hidden"))))

(fn ConstructionScript)