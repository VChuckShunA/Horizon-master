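; CheckpointBP is a kart racing checkpoint that detects when a vehicle passes through it in the correct direction.
; When a VehiclePawn leaves the trigger volume, the dot product of its velocity and the Arrow component's forward vector confirms forward travel.
; A valid pass fires the CheckpointCleared dispatcher with the checkpoint number, then hides the trigger and particle effect and disables further overlap events.
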(event OnComponentEndOverlap(Trigger)
  (params (OverlappedComponent :type Primitive%20Component%20Object%20Reference) (OtherActor :type Actor%20Object%20Reference) (OtherComp :type Primitive%20Component%20Object%20Reference) (OtherBodyIndex :type Integer))
  (bind _trigger (Variables|Default|GetTrigger))
  ;[1 1 1] Cleared when overlapping Ends
  (bind _asvehicle_pawn (Utilities|Casting|CastToVehiclePawn OtherActor))
  (if (> (Math|Vector|DotProduct (Transformation|GetVelocity _asvehicle_pawn) (Math|Rotator|GetRotationXVector (Transformation|GetWorldRotation (Variables|Default|GetArrow)))) 0.0)
    (Default|CallOnCheckpointCleared (Variables|Default|GetCheckpointNumber))
    (Development|SetHiddeninGame _trigger true false)
    (Variables|/Script/Engine.PrimitiveComponent|SetbGenerateOverlapEvents _trigger false)))

(fn ConstructionScript)