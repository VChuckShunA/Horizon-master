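; Vendor character Blueprint that supplies a list of items to the player's vendor inventory widget.
; On BeginPlay it casts the first player character to HorizonCharacterBP and caches the reference.
; The InitializeInventory event adds each VendorItems entry to that character's WVendorInventory, printing its item class name, then updates the widget with the full list.
; Nothing in this Blueprint calls InitializeInventory, and overlap and Tick are unused.
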(event Collision|EventActorBeginOverlap
  (params (OtherActor :type Actor%20Object%20Reference)))

(event EventTick
  (params (DeltaSeconds :type Float%20%28single-precision%29)))

(event EventInitializeInventory
  (bind _characterbp (Variables|Default|GetCharacterBP))
  (bind _vendoritems (Variables|Default|GetVendorItems))
  (bind _w_vendorinventory (Variables|/Game/_Game/Character/HorizonCharacterBP.HorizonCharacterBP_C|GetW_VendorInventory _characterbp))
  (for _array_element _vendoritems
    (Development|PrintString (Utilities|GetClassDisplayName (.ItemClass (Utilities|Struct|BreakItemData _array_element))))
    (Default|AddItem _w_vendorinventory _array_element))
  (Default|Update _w_vendorinventory _vendoritems))

(event EventBeginPlay
  (bind _ashorizon_character_bp (Utilities|Casting|CastToHorizonCharacterBP (Game|GetPlayerCharacter 0)))
  (Variables|Default|SetCharacterBP _ashorizon_character_bp))

(fn ConstructionScript)