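; Weather controller Blueprint that toggles between a clear bright sky and a dark, rainy one on left mouse click.
; A FlipFlop plays or reverses a timeline that lerps sky material colors, cloud opacity and light color when playing or rewinding.
; Rain particles activate five seconds after darkening starts, and deactivate five seconds before the sky starts to clear.
; The BeginPlay timer event is an empty stub.
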(event Custom|CustomEvent_0)

(event EventBeginPlay
  (Utilities|Time|SetTimerbyEvent (delegate Custom|CustomEvent_0) 0.0))

(event Input|MouseEvents|LeftMouseButton
  (params (Key :type Key%20Structure :default "None"))
  (bind _skyref (Variables|Default|GetSkyRef))
  (bind _rainref (Variables|Default|GetRainRef))
  (bind _sky_material (Variables|/Engine/EngineSky/BP_Sky_Sphere.BP_Sky_Sphere_C|GetSky%20material _skyref))
  (bind _particlesystemcomponent (Variables|/Script/Engine.Emitter|GetParticleSystemComponent _rainref))
  (:Pressed
    (if (Utilities|IsValid (Variables|Default|GetSkyRef))
      (Utilities|FlowControl|FlipFlop
        (:A
          (Utilities|FlowControl|Sequence
            (:then_0
              (bind _newtrack_0 (Timeline|Timeline_0 Play)
                (:Update
                  (Rendering|Material|SetVectorParameterValue _sky_material "Zenith Color" (Math|Color|Lerp(LinearColor) "(R=0.000000,G=0.014915,B=0.755208,A=1.000000)" "(R=0.020833,G=0.020833,B=0.020833,A=1.000000)" _newtrack_0) :!class /Script/Engine.MaterialInstanceDynamic)
                  (Rendering|Material|SetVectorParameterValue _sky_material "Horizon Color" (Math|Color|Lerp(LinearColor) "(R=1.979559,G=2.586644,B=3.000000,A=1.000000)" "(R=0.005208,G=0.005208,B=0.005208,A=1.000000)" _newtrack_0) :!class /Script/Engine.MaterialInstanceDynamic)
                  (Rendering|Material|SetVectorParameterValue _sky_material "Cloud Color" (Math|Color|Lerp(LinearColor) "(R=2.650614,G=2.845309,B=3.000000,A=1.000000)" "(R=0.005208,G=0.005208,B=0.005208,A=1.000000)" _newtrack_0) :!class /Script/Engine.MaterialInstanceDynamic)
                  (Rendering|Material|SetScalarParameterValue _sky_material "Cloud Opacity" (Math|Float|Lerp 0.2 5.0 _newtrack_0) :!class /Script/Engine.MaterialInstanceDynamic)
                  (Rendering|Components|Light|SetLightColor (Variables|/Script/Engine.Light|GetLightComponent (Variables|Default|GetLightRef)) (Math|Color|Lerp(LinearColor) "(R=2.650614,G=2.845309,B=3.000000,A=1.000000)" "(R=0.000000,G=0.000000,B=0.000000,A=1.000000)" _newtrack_0) true))))
            (:then_1
              (Utilities|FlowControl|Delay 5.0)
              (Components|Activation|Activate _particlesystemcomponent false))))
        (:B
          (Components|Activation|Deactivate _particlesystemcomponent)
          (Utilities|FlowControl|Delay 5.0)
          (Timeline|Timeline_0 Reverse))))))

(fn ConstructionScript)